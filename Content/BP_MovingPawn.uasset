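; BP_MovingPawn is a pawn that moves forward along its own facing at an adjustable speed.
; On Tick, only with authority, it sets the static mesh's physics linear velocity to the actor forward vector times Speed, replacing the current velocity.
; The IA_Move Enhanced Input action adds its scaled Y value to Speed through a SetSpeed event each time it triggers, so input accumulates.
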(event `self.ReceiveBeginPlay`)

(event `self.ReceiveTick`
  (params (DeltaSeconds :type "Float (single-precision)"))
  (`/Engine/EditorBlueprintResources/ActorMacros.Switch Has Authority`
    (:`Authority`
      (`PrimitiveComponent.SetPhysicsLinearVelocity` (`self.StaticMesh`) (* (`self.GetActorForwardVector`) (`self.Speed`)) false "None"))))

(event `SetSpeed`
  (params (Speed :type "Float (double-precision)"))
  (set `self.Speed` Speed))

(event `EnhancedInput|/Game/ThirdPerson/Input/Actions/IA_Move`
  (params (ActionValue :type "Vector2D Structure") (ElapsedSeconds :type "Float (double-precision)") (TriggeredSeconds :type "Float (double-precision)") (InputAction :type "InputAction Object Reference" :default "/Game/ThirdPerson/Input/Actions/IA_Move.IA_Move"))
  (:`Triggered`
    (`self.SetSpeed` (+ (`self.Speed`) (* ActionValue_Y 1000.0)))))

(fn `UserConstructionScript`)